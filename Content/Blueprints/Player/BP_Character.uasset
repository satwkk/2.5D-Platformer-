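; Side-scrolling player character with double jump and traversal on ledges, ropes and poles, re-locked to a fixed Y on landing or detaching.
; While jumping, Tick sphere-traces down then forward for "Grab"-tagged ledges and snaps the capsule to them in Flying mode.
; Attach events reset jumps and move the capsule to the grip; Jump detaches, and rope input flips the facing side.
; Fall-height damage detection exists but is never run.
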(event Custom|OnAttach
  (params (Attach%20Location :type Vector) (DisableInput :type Boolean))
  ;[1 0 0.3958] Event called when player attaches to something
  (Variables|Default|SetAttach%20Location Attach%20Location)
  (Variables|Default|SetIs%20Attached%20To%20Ledge true)
  (Variables|Default|SetJump%20Count 0)
  (Variables|/Script/Engine.MovementComponent|SetVelocity (Variables|Character|GetCharacterMovement) "0, 0, 0")
  (if DisableInput
    (Variables|Default|SetCan%20Move false)
    (Components|MoveComponentTo (Variables|Collision|GetCapsuleComponent) (Variables|Default|GetAttach%20Location) (Class|CharacterMovementComponent|GetLastUpdateRotation (Variables|Character|GetCharacterMovement)) false false 0.2 false)))

(event Custom|OnDetach
  ;[0 0.9387 1] Event called when player detaches from the attached actor
  (Pawn|Components|CharacterMovement|SetMovementMode (Variables|Character|GetCharacterMovement) "MOVE_Walking" 0)
  (Variables|Default|SetCan%20Move true)
  (Variables|Default|SetIs%20Attached%20To%20Ledge false)
  (Variables|Default|SetIsAttachedToRope false)
  (Variables|Default|SetIs%20Attached%20To%20Pole false)
  (Variables|Default|SetJump%20Force 5e+02)
  (Utilities|FlowControl|Delay 0.3)
  (Collision|SetCollisionResponsetoAllChannels (Variables|Collision|GetCapsuleComponent) "ECR_Block")
  (Variables|Default|SetJump%20Force 3.5e+02)
  (CallFunction|LockYAxis))

(event Custom|OnLandPole
  (params (LandLocation :type Vector))
  ;[0 1 0.08449] Event  called when player lands on a pole
  (CallFunction|OnAttach LandLocation true)
  (Variables|Default|SetIs%20Attached%20To%20Pole true)
  (Variables|/Script/Engine.CharacterMovementComponent|SetMaxWalkSpeed (Variables|Character|GetCharacterMovement) 1e+02))

(event Custom|OnAttachToRope
  (params (Attach%20Location :type Vector) (Socket%20Name :type Name))
  ;[0 1 0.8682] Event called when attached to rope
  (Components|MoveComponentTo (Variables|Collision|GetCapsuleComponent) Attach%20Location (Class|CharacterMovementComponent|GetLastUpdateRotation (Variables|Character|GetCharacterMovement)) false false 0.1 false)
  (Components|Movement|StopMovementImmediately (Variables|Character|GetCharacterMovement))
  (CallFunction|ChangeMovementMode "MOVE_Flying")
  (Variables|Default|SetCan%20Move false)
  (Variables|Default|SetIsAttachedToRope true)
  (Variables|Default|SetJump%20Count 0))

(event Custom|OnAttachToRopeTurnToInputDirection
  (bind _returnvalue (Transformation|GetActorForwardVector))
  (bind _returnvalue_2 (Transformation|GetActorLocation))
  (bind _returnvalue_3 (Transformation|GetActorRotation))
  (bind _returnvalue_4 (Input|AxisValues|GetMovement))
  (bind _returnvalue_5 (Math|Vector|MakeVector _returnvalue_4 0.0 0.0))
  (bind _returnvalue_6 (Math|Vector|DotProduct _returnvalue _returnvalue_5))
  ;[0.6956 1 0] Called in tick if player is attached to rope to rotate and change direction around the rope
  (if (> _returnvalue_6 0.0)
    ;;[1 0.3168 0] Go to right side of rope and turn to left
    (Development|PrintString (Utilities|String|ToString(Float) _returnvalue_6))
    (Transformation|SetActorLocation (Math|Vector|Lerp(Vector) _returnvalue_2 (+ _returnvalue_2 (* (Transformation|GetActorForwardVector) 2.0)) (* (Utilities|Time|GetWorldDeltaSeconds) 5e+01)) false false)
    (Utilities|FlowControl|Delay 0.2)
    (if (Math|Float|NearlyEqual(Float) (Math|Float|Absolute(Float) (.yaw _returnvalue_3)) 1.8e+02 2.0)
      (Transformation|SetWorldRotation (Variables|Collision|GetCapsuleComponent) (Math|Rotator|MakeRotator (.roll _returnvalue_3) (.pitch _returnvalue_3) 0.0) false false)
      (Development|PrintString "Rotating to 0")
      (else
        (Transformation|SetWorldRotation (Variables|Collision|GetCapsuleComponent) (Math|Rotator|MakeRotator (.roll _returnvalue_3) (.pitch _returnvalue_3) -1.8e+02) false false)
        (Development|PrintString "Rotating to -180")))))

(event Custom|Change%20Movement%20Mode
  (params (Movement%20Mode :type EMovementMode%20Enum :default "MOVE_None"))
  (bind _charactermovement (Variables|Character|GetCharacterMovement))
  ;[1 0.4037 0.6722] Event Called by other classes to change the movement mode of this actor
  (Pawn|Components|CharacterMovement|SetMovementMode _charactermovement Movement%20Mode 0)
  (if (Utilities|Enum|Equal(Enum) Movement%20Mode "MOVE_Flying")
    (Components|Movement|StopMovementImmediately _charactermovement)))

(event EventBeginPlay
  (CallFunction|SetupVariablesandReferences))

(event EventOnLanded
  (params (Hit :type Hit%20Result%20Structure%20%28by%20ref%29))
  ;[1 0.2991 0] Jump and On Land
  (Variables|Default|SetJump%20Count 0)
  (Variables|/Script/Engine.CharacterMovementComponent|SetMaxWalkSpeed (Variables|Character|GetCharacterMovement) 4e+02)
  (Variables|Default|SetIs%20Jumping false)
  (CallFunction|LockYAxis))

(event EventTick
  (params (DeltaSeconds :type Float%20%28single-precision%29))
  (bind _charactermovement (Variables|Character|GetCharacterMovement))
  (bind _wallgraboffset (Variables|ParkourVals|GetWallGrabOffset))
  ;[0 0.3481 1] Tick
  (Utilities|FlowControl|Sequence
    (:then_0
      (if (Variables|Default|GetIs%20Attached%20To%20Ledge)
        _))
    (:then_1
      (if (Variables|Default|GetIsAttachedToRope)
        (CallFunction|OnAttachtoRopeTurntoInputDirection)))
    (:then_2
      (if (and (Variables|Default|GetIs%20Jumping) (Variables|Default|GetCanRaycast))
        (bind _grab_location (CallFunction|LineTraceforGrab))
        (if (<= (Math|Vector|Distance(Vector) (Transformation|GetActorLocation) _grab_location) 9e+01)
          (Variables|Default|SetCan%20Move false)
          (Variables|Default|SetIs%20Attached%20To%20Ledge true)
          (Development|PrintString "Can Grab")
          (Transformation|SetWorldLocation (Variables|Collision|GetCapsuleComponent) (Math|Vector|Lerp(Vector) (Transformation|GetWorldLocation (Variables|Collision|GetCapsuleComponent)) (Math|Vector|MakeVector (- (.X (Math|Vector|BreakVector _grab_location)) (.x _wallgraboffset)) (.Y (Math|Vector|BreakVector _grab_location)) (- (.Z (Math|Vector|BreakVector _grab_location)) (.y _wallgraboffset))) (* (Utilities|Time|GetWorldDeltaSeconds) 1e+01)) false false)
          (Utilities|FlowControl|Delay 0.1)
          (Pawn|Components|CharacterMovement|SetMovementMode _charactermovement "MOVE_Flying" 0)
          (Components|Movement|StopMovementImmediately _charactermovement))))))

(event Input|ActionEvents|InputActionJump
  (params (Key :type Key%20Structure :default "None"))
  ;[1 0.2991 0] Jump and On Land
  (:Pressed
    (Utilities|FlowControl|Sequence
      (:then_0
        (if (Math|Boolean|ORBoolean (Variables|Default|GetIs%20Attached%20To%20Ledge) (Variables|Default|GetIsAttachedToRope) (Variables|Default|GetIs%20Attached%20To%20Pole))
          (CallFunction|OnDetach)
          (Variables|Default|SetCanRaycast false)
          (Utilities|FlowControl|Delay 2.0)
          (Variables|Default|SetCanRaycast true)))
      (:then_1
        (if (< (Variables|Default|GetJump%20Count) 2)
          (Character|LaunchCharacter (* (Transformation|GetActorUpVector) (Variables|Default|GetJump%20Force)) false false)
          (bind _result (Math|Integer|IncrementInt (Variables|Default|GetJump%20Count))
            (:%20%20
              (Variables|Default|SetJump%20Count _result)
              (Variables|Default|SetIs%20Jumping true))))))))

(event Input|AxisEvents|InputAxisMovement
  (params (AxisValue :type Float%20%28single-precision%29))
  (bind _returnvalue (Input|AxisValues|GetMovement))
  ;[0 1 0.7507] Movement
  (Variables|Default|SetMovementInput _returnvalue)
  (if (Variables|Default|GetCan%20Move)
    (Pawn|Input|AddMovementInput self (Math|Transform|InverseTransformDirection (Transformation|GetActorTransform) (Transformation|GetActorForwardVector)) (* _returnvalue (Utilities|Time|GetWorldDeltaSeconds) (Variables|/Script/Engine.CharacterMovementComponent|GetMaxWalkSpeed (Variables|Character|GetCharacterMovement))) false)))

(fn ConstructionScript)

(fn SetupVariablesandReferences
  (bind _mesh (Variables|Character|GetMesh))
  (bind _returnvalue (Components|SkeletalMesh|GetAnimInstance _mesh))
  (Utilities|FlowControl|Sequence
    (:then_0
      ;[1 1 1] Caching the controller
      (bind _asbp_player_controller (Utilities|Casting|CastToBP_PlayerController (Pawn|GetController))
        (:then
          (Variables|Default|SetPlayerController _asbp_player_controller))
        (:CastFailed
          (Development|PrintString "Controller cast failed"))))
    (:then_1
      ;[1 1 1] Caching the animation blueprint
      (if (Utilities|IsValid _returnvalue)
        (bind _asabp_character (Utilities|Casting|CastToABP_Character _returnvalue))
        (if (Utilities|IsValid _asabp_character)
          (Variables|Default|SetAnimationBP _asabp_character)
          (else
            (Development|PrintString "Animation BP Casting failed")))))))

(fn AttachtoLedge
  (params (Ledge :type BP%20Ledge%20Object%20Reference) (SocketName :type Name))
  (CallFunction|OnAttach (Transformation|GetSocketLocation (Variables|/Game/Blueprints/Ledge/BP_Ledge.BP_Ledge_C|GetMesh Ledge) SocketName) true))

(fn LerptoLedgeSocket
  (Transformation|SetActorLocation (Math|Vector|Lerp(Vector) (Transformation|GetActorLocation) (Variables|Default|GetAttach%20Location) (* (Utilities|Time|GetWorldDeltaSeconds) (Variables|Default|GetLedgeAttachSnappiness))) false false))

(fn LandonPole
  (params (Pole :type BP%20Pole%20Object%20Reference))
  (CallFunction|OnLandPole (Variables|/Game/Blueprints/Pole/BP_Pole.BP_Pole_C|GetPlayerLandLocation Pole)))

(fn IsFacingAttachActorDirection
  (bind _returnvalue (Transformation|GetActorForwardVector))
  (bind _charactermovement (Variables|Character|GetCharacterMovement))
  (bind _returnvalue_2 (Pawn|Components|CharacterMovement|GetLastUpdateVelocity _charactermovement))
  (bind _returnvalue_3 (Math|Vector|Normalize _returnvalue_2))
  (bind _returnvalue_4 (Math|Vector|DotProduct _returnvalue_3 _returnvalue))
  (Development|PrintString (Utilities|String|ToString(Float) _returnvalue_4))
  (return (>= _returnvalue_4 0.1)))

(fn FallHeightCheck
  (bind _returnvalue (Transformation|GetActorLocation))
  (if (< (.z (Variables|/Script/Engine.MovementComponent|GetVelocity (Variables|Character|GetCharacterMovement))) 0.0)
    (bind _outhit (Collision|LineTraceByChannel _returnvalue (+ _returnvalue (* (* (Transformation|GetActorUpVector) -1.0) 1e+03)) "TraceTypeQuery1" false 0 "ForOneFrame" true "(R=1.000000,G=0.000000,B=0.000000,A=1.000000)" "(R=0.000000,G=1.000000,B=0.000000,A=1.000000)" 1.0))
    (if (> (Math|Vector|Distance(Vector) (Transformation|GetActorLocation) (.location _outhit)) (Variables|Default|GetMax%20Height))
      (bind _output_get (Variables|Default|SetMax%20Height (Math|Vector|Distance(Vector) (Transformation|GetActorLocation) (.location _outhit))))
      (Development|PrintString (Utilities|String|ToString(Float) _output_get))
      (if (> _output_get (Variables|Default|GetFallDamageHeight))
        (bind _output_get_2 (Variables|Default|SetCan%20Be%20Damaged%20By%20Fall true))
        (else
          (Variables|Default|SetCan%20Be%20Damaged%20By%20Fall false)))
      (Development|PrintString (Utilities|String|ToString(Boolean) _output_get_2)))))

(fn LockYAxis
  (bind _returnvalue (Transformation|GetActorLocation))
  (Transformation|SetActorLocation (Math|Vector|MakeVector (.x _returnvalue) 9e+01 (.z _returnvalue)) false false))

(fn LineTraceforGrab
  (bind _returnvalue (Transformation|GetActorLocation))
  (bind _returnvalue_2 (Transformation|GetActorForwardVector))
  (bind _returnvalue_3 (Transformation|GetActorLocation))
  (bind _grabdistance (Variables|ParkourVals|GetGrabDistance))
  (bind _downtraceheight (Variables|ParkourVals|GetDownTraceHeight))
  (bind _returnvalue_4 (* _returnvalue_2 _grabdistance))
  (bind _returnvalue_5 (+ (.z _returnvalue_4) _downtraceheight))
  (bind _returnvalue_6 (+ _returnvalue (Math|Vector|MakeVector (.x _returnvalue_4) (.y _returnvalue_4) _returnvalue_5)))
  ;[0.1615 0.1615 0.1615] Down Trace
  (bind _outhit (Collision|SphereTraceByChannel _returnvalue_6 (+ _returnvalue_6 (* (Math|Vector|VectorDown) (Variables|ParkourVals|GetDownTraceRange))) 1e+01 "TraceTypeQuery1" false (Utilities|Array|MakeArray self) "ForOneFrame"))
  (Variables|ParkourVals|SetDownTraceHitResult _outhit)
  ;[0.04519 0.04519 0.04519] Forward Trace
  (bind _outhit_2 (Collision|SphereTraceByChannel (Math|Vector|MakeVector (.x _returnvalue_3) (.y _returnvalue_3) (+ (.z (.location (Variables|ParkourVals|GetDownTraceHitResult))) -1.0)) (+ (Math|Vector|MakeVector (.x _returnvalue_3) (.y _returnvalue_3) (+ (.z (.location (Variables|ParkourVals|GetDownTraceHitResult))) -1.0)) (* (Transformation|GetActorForwardVector) 1e+02)) 1e+01 "TraceTypeQuery1" false (Utilities|Array|MakeArray self) "ForOneFrame" true "(R=0.000000,G=0.441897,B=1.000000,A=1.000000)"))
  (Rendering|Debug|DrawDebugSphere (.location _outhit_2) 15.0 12 "(R=1.000000,G=1.000000,B=1.000000,A=1.000000)" 0.0)
  (if (Utilities|Array|ContainsItem (Variables|/Script/Engine.Actor|GetTags (.hitactor _outhit_2)) "Grab")
    (return (.location _outhit_2))))