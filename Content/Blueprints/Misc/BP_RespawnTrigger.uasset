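; BP_RespawnTrigger is a box trigger that sends the player back to their current checkpoint on overlap, costing one life.
; BeginPlay caches the first BP_Character and its starting location.
; Overlap checks that character's lives, then teleports it and decrements Lives, or only prints a death message when none remain.
; The checkpoint helper with a start-location fallback is unused, so the checkpoint is read without a validity check.
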(event OnComponentBeginOverlap(Box)
  (params (OverlappedComponent :type Primitive%20Component%20Object%20Reference) (OtherActor :type Actor%20Object%20Reference) (OtherComp :type Primitive%20Component%20Object%20Reference) (OtherBodyIndex :type Integer) (bFromSweep :type Boolean) (SweepResult :type Hit%20Result%20Structure%20%28by%20ref%29))
  (if (Utilities|IsValid OtherActor)
    (bind _asbp_character (Utilities|Casting|CastToBP_Character OtherActor))
    (if (Utilities|IsValid _asbp_character)
      (if (== _asbp_character (Variables|Default|GetPlayer))
        (bind _haslives (CallFunction|DoesPlayerHaveLives))
        (if _haslives
          (Transformation|SetActorLocation (Variables|Default|GetPlayer) (Transformation|GetActorLocation (Variables|/Game/Blueprints/Player/BP_Character.BP_Character_C|GetCurrent%20CheckPoint (Variables|Default|GetPlayer))) false false)
          (Math|Integer|DecrementInt (Variables|/Game/Blueprints/Player/BP_Character.BP_Character_C|GetLives (Variables|Default|GetPlayer)))
          (else
            (Development|PrintString "You are dead")))))))

(event EventBeginPlay
  (bind _returnvalue (Actor|GetActorOfClass "/Game/Blueprints/Player/BP_Character.BP_Character_C"))
  (if (Utilities|IsValid _returnvalue)
    (bind _output_get (Variables|Default|SetPlayer _returnvalue))
    (Variables|Default|SetInitial%20Player%20Location (Transformation|GetActorLocation _output_get))))

(event Collision|EventActorBeginOverlap
  (params (OtherActor :type Actor%20Object%20Reference)))

(event EventTick
  (params (DeltaSeconds :type Float%20%28single-precision%29)))

(fn ConstructionScript)

(fn GetActorCurrentCheckPointLocation
  (bind _player (Variables|Default|GetPlayer))
  (bind _current_checkpoint (Variables|/Game/Blueprints/Player/BP_Character.BP_Character_C|GetCurrent%20CheckPoint _player))
  (if (Utilities|IsValid _current_checkpoint)
    (return (Transformation|GetActorLocation _current_checkpoint))
    (else
      (return (Variables|Default|GetInitial%20Player%20Location)))))

(fn DoesPlayerHaveLives
  (if (> (Variables|/Game/Blueprints/Player/BP_Character.BP_Character_C|GetLives (Variables|Default|GetPlayer)) 0)
    (return true)
    (else
      (return false))))