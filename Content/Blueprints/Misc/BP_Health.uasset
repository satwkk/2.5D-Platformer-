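; BP_Health is a pickup actor that grants the player an extra life on overlap.
; When its Box trigger overlaps a BP_Character, it increments that character's Lives and prints a debug message.
; It then hides the Mesh and disables collision on both Box and Mesh, leaving the actor in the level instead of destroying it.
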(event OnComponentBeginOverlap(Box)
  (params (OverlappedComponent :type Primitive%20Component%20Object%20Reference) (OtherActor :type Actor%20Object%20Reference) (OtherComp :type Primitive%20Component%20Object%20Reference) (OtherBodyIndex :type Integer) (bFromSweep :type Boolean) (SweepResult :type Hit%20Result%20Structure%20%28by%20ref%29))
  ;[1 0 0.01975] Increments player health when player overlaps with this actor
  (if (Utilities|IsValid OtherActor)
    (bind _asbp_character (Utilities|Casting|CastToBP_Character OtherActor))
    (if (Utilities|IsValid _asbp_character)
      (Math|Integer|IncrementInt (Variables|/Game/Blueprints/Player/BP_Character.BP_Character_C|GetLives _asbp_character)
        (:%20%20
          (Development|PrintString "Incrementing Lives")
          (Rendering|SetVisibility (Variables|Default|GetMesh) false false)
          (Collision|SetCollisionEnabled (Variables|Default|GetBox) "NoCollision")
          (Collision|SetCollisionEnabled (Variables|Default|GetMesh) "NoCollision"))))))

(event EventBeginPlay)

(event Collision|EventActorBeginOverlap
  (params (OtherActor :type Actor%20Object%20Reference)))

(event EventTick
  (params (DeltaSeconds :type Float%20%28single-precision%29)))

(fn ConstructionScript)