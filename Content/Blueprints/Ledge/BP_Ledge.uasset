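; BP_Ledge is a ledge actor that BP_Character can grab from a left or right attach trigger.
; On overlap, each trigger casts to BP_Character and asks it whether it is facing the attach direction.
; If so, the character attaches to the ledge at that side's named socket and switches to Flying movement; otherwise a debug message prints.
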(event OnComponentBeginOverlap(AttachTrigger_L)
  (params (OverlappedComponent :type Primitive%20Component%20Object%20Reference) (OtherActor :type Actor%20Object%20Reference) (OtherComp :type Primitive%20Component%20Object%20Reference) (OtherBodyIndex :type Integer) (bFromSweep :type Boolean) (SweepResult :type Hit%20Result%20Structure%20%28by%20ref%29))
  ;[1 0 0.04113] On Left Trigger Overlap
  (Utilities|IsValid OtherActor
    (:Is%20Valid
      (bind _asbp_character (Utilities|Casting|CastToBP_Character OtherActor))
      (Utilities|IsValid _asbp_character
        (:Is%20Valid
          (bind _isfacing (Default|IsFacingAttachActorDirection _asbp_character))
          (if _isfacing
            (Default|AttachtoLedge _asbp_character self (Variables|Default|GetL_SKT_Name))
            (Default|ChangeMovementMode _asbp_character "MOVE_Flying")
            (else
              (Development|PrintString "Not Facing L"))))))))

(event OnComponentBeginOverlap(AttachTrigger_R)
  (params (OverlappedComponent :type Primitive%20Component%20Object%20Reference) (OtherActor :type Actor%20Object%20Reference) (OtherComp :type Primitive%20Component%20Object%20Reference) (OtherBodyIndex :type Integer) (bFromSweep :type Boolean) (SweepResult :type Hit%20Result%20Structure%20%28by%20ref%29))
  ;[0 0.2203 1] On Right Trigger Overlap
  (Utilities|IsValid OtherActor
    (:Is%20Valid
      (bind _asbp_character (Utilities|Casting|CastToBP_Character OtherActor))
      (Utilities|IsValid _asbp_character
        (:Is%20Valid
          (bind _isfacing (Default|IsFacingAttachActorDirection _asbp_character))
          (if _isfacing
            (Default|AttachtoLedge _asbp_character self (Variables|Default|GetR_SKT_Name))
            (Default|ChangeMovementMode _asbp_character "MOVE_Flying")
            (else
              (Development|PrintString "Not Facing R"))))))))

(event EventBeginPlay)

(event Collision|EventActorBeginOverlap
  (params (OtherActor :type Actor%20Object%20Reference)))

(event EventTick
  (params (DeltaSeconds :type Float%20%28single-precision%29)))

(fn ConstructionScript)