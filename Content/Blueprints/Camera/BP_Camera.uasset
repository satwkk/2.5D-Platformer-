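; BP_Camera is a side-scrolling style follow camera that tracks the BP_Character actor.
; On BeginPlay it finds the character, enables following and stores its own initial location.
; Each Tick, while following is enabled, it moves to the character's X plus a small offset and matches its Z, keeping its starting Y fixed.
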(event EventBeginPlay
  (bind _returnvalue (Actor|GetActorOfClass "/Game/Blueprints/Player/BP_Character.BP_Character_C"))
  (Variables|Default|SetFollowTarget _returnvalue)
  (Variables|Default|SetCanFollow true)
  (Variables|Default|SetCamera%20Initial%20Location (Transformation|GetActorLocation)))

(event Collision|EventActorBeginOverlap
  (params (OtherActor :type Actor%20Object%20Reference)))

(event EventTick
  (params (DeltaSeconds :type Float%20%28single-precision%29))
  (bind _followtarget (Variables|Default|GetFollowTarget))
  (bind _returnvalue (Transformation|GetActorLocation _followtarget))
  (if (Variables|Default|GetCanFollow)
    (Transformation|SetActorLocation (Math|Vector|MakeVector (+ (.x _returnvalue) 5e+01) (.y (Variables|Default|GetCamera%20Initial%20Location)) (.z _returnvalue)) false false)))

(fn ConstructionScript)